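; BP_ImGuiTest is a test Blueprint that draws a sample Dear ImGui window to exercise the plugin's Blueprint widget nodes.
; BeginPlay enlarges the UI scale, and Tick rebuilds the fixed window at the viewport's top-right each frame.
; Widgets bind to Blueprint variables inside tree nodes and a collapsing header, where radio buttons switch between an integer slider and a line plot.
; The DialogTest node is empty.
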(event EventBeginPlay
  (|CallParentFunction)
  (Class|BPImGui|ScaleAllSizes 1.2))

(event EventTick
  (params (DeltaSeconds :type Float%20%28single-precision%29))
  (bind _array (Utilities|Array|MakeArray 0.0 2345.0 2e+01 0.234 234.0 2.0 235.0 2.0 23.0 1.54))
  (bind _radio (Variables|Default|GetRadio))
  (|CallParentFunction 0.0)
  (Class|BPImGui|BeginGUI "Test" (Math|Vector2D|MakeVector2D (.x (Viewport|GetViewportSize)) 0.0) "(X=1.000000,Y=0.000000)" "(X=300.000000,Y=700.000000)" (Utilities|Struct|MakeImGuiWindowFlags false false true))
  (Class|BPImGui|AddSliderFloat "Slider" (Variables|Default|GetValue) 0.0 1.0)
  (Utilities|FlowControl|Sequence
    (:then_0
      (bind _returnvalue (Class|BPImGui|BeginTreeNodes "TreeTest" true))
      (if _returnvalue
        (Class|BPImGui|AddCombo "Combo" (Variables|Default|GetComboItem) (Utilities|Array|MakeArray "abc" "ljbnuo" "sgh"))
        (Class|BPImGui|AddListBox "List" (Variables|Default|GetListItem) (Utilities|Array|MakeArray "abc" "ljbnuo" "sgh") 4)
        (Class|BPImGui|AddTextInput "Input" (Variables|Default|GetTextInput) 64)
        (Class|BPImGui|AddColor "Color" (Variables|Default|GetColor))
        (Class|BPImGui|EndTreeNode)))
    (:then_1
      (bind _returnvalue_2 (Class|BPImGui|BeginTreeNodes "DialogTest" true))
      (if _returnvalue_2
        (Class|BPImGui|EndTreeNode)))
    (:then_2
      (bind _returnvalue_3 (Class|BPImGui|CollapsingHeader "Header" true))
      (if _returnvalue_3
        (Class|BPImGui|AddBulletText "Bullet Text")
        (Class|BPImGui|AddDragIntRange "Range" (Variables|Default|GetV_0) 1 0 150)
        (Class|BPImGui|AddRadioButton "Item1" _radio)
        (Class|BPImGui|SameLine 0.0 -1.0)
        (Class|BPImGui|AddRadioButton "Item2" _radio 1)
        (if (== _radio 0)
          (Class|BPImGui|AddSliderInt3 "Slider Int3" (Variables|Default|GetV) 0 20)
          (else
            (Class|BPImGui|PlotLines "Lines" _array (Utilities|Array|Length _array))))))
    (:then_3
      (Class|BPImGui|AddText "End")
      (Class|BPImGui|EndGUI))))

(fn ConstructionScript
  (|CallParentFunction))